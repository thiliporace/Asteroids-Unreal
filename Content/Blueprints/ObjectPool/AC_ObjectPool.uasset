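; Actor component that keeps a pool of pre-spawned actors for reuse.
; On BeginPlay it spawns actors of PooledActorClass up to PoolSize, passing each a LifeTime and marking it not in use.
; SpawnFromPool finds the first valid idle actor by linear search, moves it to the requested transform and marks it in use.
; The pool never grows, printing a message when no actor is available.
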(event Custom|InitializePool
  (for _index (range 0 (Variables|Default|GetPoolSize))
    (bind _returnvalue (Game|SpawnActorfromClass (Variables|Default|GetPooledActorClass) (Variables|Default|GetTransform) "Undefined" "MultiplyWithRoot" 0 (Variables|Default|GetLife%20Time) 0))
    (Utilities|Array|AddUnique (Variables|Default|GetObjectPool) _returnvalue)
    (Default|SetinUse _returnvalue false)))

(event EventBeginPlay
  (CallFunction|InitializePool))

(event EventTick
  (params (DeltaSeconds :type Float%20%28single-precision%29)))

(fn FindFirstAvailableActor
  (for _array_element (Variables|Default|GetObjectPool)
    (Utilities|IsValid _array_element
      (:Is%20Valid
        (if (not (Variables|/Game/Blueprints/ObjectPool/BP_PooledActor.BP_PooledActor_C|GetInUse _array_element))
          (return _array_element))))))

(fn SpawnfromPool
  (params (SpawnTransform :type Transform))
  (bind _pooledactor (CallFunction|FindFirstAvailableActor))
  (if (Utilities|IsValid _pooledactor)
    (Transformation|SetActorTransform _pooledactor SpawnTransform)
    (Default|SetinUse _pooledactor true)
    (return _pooledactor)
    (else
      (Development|PrintString "actor trying to be spawned isn't valid"))))