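; BP_LifeSystemComponent is a component that tracks health for its owner and handles death.
; On BeginPlay it fills Health to MaxHealth and blocks damage for an InvincibilityTimer delay, giving a spawn grace period.
; TakeDamage subtracts from Health only while damage is allowed, and calls the KillYourself dispatcher when Health reaches zero or below, leaving the death response to listeners.
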(event EventBeginPlay
  (Variables|Default|Sethealth (Variables|Default|GetmaxHealth))
  (Variables|Default|SetcanTakeDamage false)
  (Utilities|FlowControl|Delay (Variables|Default|GetinvincibilityTimer))
  (Variables|Default|SetcanTakeDamage true))

(event EventTick
  (params (DeltaSeconds :type Float%20%28single-precision%29)))

(event EventTakeDamage
  (params (damage :type Integer))
  (if (Variables|Default|GetcanTakeDamage)
    (bind _output_get (Variables|Default|Sethealth (- (Variables|Default|Gethealth) damage)))
    (if (<= _output_get 0)
      (Default|CallKillYourselfDispatcher))))