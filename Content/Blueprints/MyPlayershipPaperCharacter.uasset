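; Paper2D character Blueprint for the player ship, tracking rotate, move and shoot state from Enhanced Input actions.
; Rotating and moving are mutually exclusive: each action sets its flag only while the other is inactive and clears it on completion.
; The shoot action raises a shooting flag, then lowers it after a configurable delay between shots.
; The graph only sets these state flags, with no movement or bullet-spawning logic of its own.
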(event Input|EnhancedActionEvents|EnhancedInputActionIA_Rotate
  (params (ActionValue :type Float%20%28double-precision%29) (ElapsedSeconds :type Float%20%28double-precision%29) (TriggeredSeconds :type Float%20%28double-precision%29) (InputAction :type Input%20Action%20Object%20Reference :default "/Game/Input/IA_Rotate.IA_Rotate"))
  (:Triggered
    (if (not (Variables|Default|GetisMoving))
      (Variables|Default|SetisRotating true)))
  (:Completed
    (Variables|Default|SetisRotating false)))

(event Input|EnhancedActionEvents|EnhancedInputActionIA_Move
  (params (ActionValue :type Float%20%28double-precision%29) (ElapsedSeconds :type Float%20%28double-precision%29) (TriggeredSeconds :type Float%20%28double-precision%29) (InputAction :type Input%20Action%20Object%20Reference :default "/Game/Input/IA_Move.IA_Move"))
  (:Triggered
    (if (not (Variables|Default|GetisRotating))
      (Variables|Default|SetisMoving true)))
  (:Completed
    (Variables|Default|SetisMoving false)))

(event Input|EnhancedActionEvents|EnhancedInputActionIA_ShootBullet
  (params (ActionValue :type Boolean) (ElapsedSeconds :type Float%20%28double-precision%29) (TriggeredSeconds :type Float%20%28double-precision%29) (InputAction :type Input%20Action%20Object%20Reference :default "/Game/Input/IA_ShootBullet.IA_ShootBullet"))
  (Variables|Default|SetisShooting true)
  (Utilities|FlowControl|Delay (Variables|Default|GetdelayBetweenShots))
  (Variables|Default|SetisShooting false))

(event EventBeginPlay)

(event Collision|EventActorBeginOverlap
  (params (OtherActor :type Actor%20Object%20Reference)))

(event EventTick
  (params (DeltaSeconds :type Float%20%28single-precision%29)))

(fn ConstructionScript)