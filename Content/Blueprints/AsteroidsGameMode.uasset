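; Game mode for an Asteroids game that tracks player lives and score and shows them in a HUD widget.
; On BeginPlay it creates the widget, adds it to the viewport and sets the life count.
; A death event decrements lives and respawns the player after a cooldown, or only prints a message when none remain.
; A points event adds to the total and pushes the score text to the widget.
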(event Custom|AddPoints_Event
  (params (Points :type Integer))
  (bind _output_get (Variables|Default|SetTotalPoints (+ (Variables|Default|GetTotalPoints) Points)))
  (Default|SetTextEvent (Variables|Default|GetWidget%20Blueprint) (Utilities|String|ToString(Integer) _output_get)))

(event Custom|PlayerDied_Event
  (params (NewParam :type Controller%20Object%20Reference))
  (bind _output_get (Variables|Default|SetPlayerLives (- (Variables|Default|GetPlayerLives) 1)))
  (Variables|/Game/Blueprints/WidgetBlueprint.WidgetBlueprint_C|SetNumLives (Variables|Default|GetWidget%20Blueprint) _output_get)
  (if (<= _output_get 0)
    (Development|PrintString "acabou as vidas")
    (else
      (Development|PrintString "player respawn")
      (Utilities|FlowControl|Delay (Variables|Default|GetrespawnCooldown))
      (Class|GameModeBase|RestartPlayer NewParam))))

(event EventBeginPlay
  (bind _returnvalue (UserInterface|CreateWidget "/Game/Blueprints/WidgetBlueprint.WidgetBlueprint_C"))
  (bind _output_get (Variables|Default|SetWidget%20Blueprint _returnvalue))
  (UserInterface|Viewport|AddtoViewport _output_get 0)
  (Variables|/Game/Blueprints/WidgetBlueprint.WidgetBlueprint_C|SetNumLives (Variables|Default|GetWidget%20Blueprint) (Variables|Default|GetPlayerLives)))

(event EventTick
  (params (DeltaSeconds :type Float%20%28single-precision%29)))

(fn ConstructionScript)