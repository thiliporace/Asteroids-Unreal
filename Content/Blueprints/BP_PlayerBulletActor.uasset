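; BP_PlayerBulletActor is the player's projectile, which damages meteors and destroys itself after BulletLifeTime if nothing ends it sooner.
; When its Sphere overlaps a Meteor-tagged component whose owner has a LifeSystemComponent, it hides the sprite, zeroes ProjectileMovement velocity and deals a fixed amount of damage.
; It plays the hit flipbook once and destroys itself after the effect's duration, computed from flipbook length and play rate.
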(event OnComponentBeginOverlap(Sphere)
  (params (OverlappedComponent :type Primitive%20Component%20Object%20Reference) (OtherActor :type Actor%20Object%20Reference) (OtherComp :type Primitive%20Component%20Object%20Reference) (OtherBodyIndex :type Integer) (bFromSweep :type Boolean) (SweepResult :type Hit%20Result%20Structure%20%28by%20ref%29))
  (bind _returnvalue (Actor|GetComponentbyClass OtherActor "/Script/Asteroids.LifeSystemComponent"))
  (bind _hiteffectflipbook (Variables|Default|GetHitEffectFlipbook))
  (bind _hiteffectflipbook_2 (Variables|Default|GetHitEffectFlipbook))
  (if (Components|ComponentHasTag OtherComp "Meteor")
    (if (Utilities|IsValid _returnvalue)
      (Rendering|SetVisibility (Variables|Default|GetPaperSprite) false false)
      (Components|Timeline|SetLooping _hiteffectflipbook_2 false)
      (Audio|Components|Audio|Play _hiteffectflipbook_2)
      (Variables|/Script/Engine.MovementComponent|SetVelocity (Variables|Default|GetProjectileMovement) "0, 0, 0")
      (Class|LifeSystemComponent|TakeDamage _returnvalue 2)
      (Utilities|FlowControl|Delay (/ (Class|PaperFlipbookComponent|GetFlipbookLength _hiteffectflipbook) (Components|Animation|GetPlayRate _hiteffectflipbook)))
      (Actor|DestroyActor))))

(event EventBeginPlay
  (|CallParentFunction)
  (Utilities|FlowControl|Delay (Variables|Default|GetbulletLifeTime))
  (Actor|DestroyActor))

(event Collision|EventActorBeginOverlap
  (params (OtherActor :type Actor%20Object%20Reference)))

(event EventTick
  (params (DeltaSeconds :type Float%20%28single-precision%29)))

(fn ConstructionScript)