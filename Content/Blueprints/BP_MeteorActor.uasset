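; BP_MeteorActor is a meteor actor with a Paper2D sprite and a limited lifetime.
; On BeginPlay it runs the parent logic, then picks a random frame from SpritesFlipbook as its sprite, using the flipbook as a pool of visual variants rather than an animation.
; It then waits for MeteorLifetime and destroys itself.
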(event EventBeginPlay
  (|CallParentFunction)
  (Rendering|Components|Sprite|SetSprite (Variables|Default|GetPaperSprite) (Class|PaperFlipbook|GetSpriteatFrame (Variables|Default|GetspritesFlipbook) (Math|Random|RandomIntegerinRange 0 (- (Class|PaperFlipbook|GetNumFrames (Variables|Default|GetspritesFlipbook)) 1))))
  (Utilities|FlowControl|Delay (Math|Conversions|ToFloat(Integer) (Variables|Default|GetmeteorLifetime)))
  (Actor|DestroyActor))

(event Collision|EventActorBeginOverlap
  (params (OtherActor :type Actor%20Object%20Reference)))

(event EventTick
  (params (DeltaSeconds :type Float%20%28single-precision%29)))

(fn ConstructionScript)